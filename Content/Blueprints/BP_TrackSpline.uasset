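; BP_TrackSpline is a track spline that AI vehicles follow, registering itself with BP_VehicleAdvGameMode as a follow target on BeginPlay when active.
; It supplies separate steering and speed target points by projecting the requesting vehicle onto the spline and looking ahead along it.
; Look-ahead distance scales with the vehicle's forward speed in km/h through a clamped range, with the speed point farther ahead than the steering point.
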(event `self.ReceiveBeginPlay`
  (`parent.ReceiveBeginPlay`)
  (if (`self.bIsActive`)
    (bind _asbp_vehicle_adv_game_mode (cast `/Game/VehicleTemplate/Blueprints/BP_VehicleAdvGameMode` (`GameplayStatics.GetGameMode`)))
    (`MadBumbumsGameMode.RegisterAsFollowTarget` _asbp_vehicle_adv_game_mode self)))

(fn `GetSpeedLocationForAI`
  (params (Requester :type "Actor Object Reference"))
  (returns (ReturnValue :type "Vector Structure"))
  (bind _spline (`self.Spline`))
  (return (`SplineComponent.GetLocationAtDistanceAlongSpline` _spline (+ (`SplineComponent.GetDistanceAlongSplineAtLocation` _spline (`self.K2_GetActorLocation` Requester) "World") (`KismetMathLibrary.MapRangeClamped` (* (`ChaosVehicleMovementComponent.GetForwardSpeed` (`self.GetComponentByClass` (`local.Requester`) "/Script/ChaosVehicles.ChaosVehicleMovementComponent")) 0.036) 50.0 230.0 2500.0 7500.0)) "World")))

(fn `GetSteerLocationForAI`
  (params (Requester :type "Actor Object Reference"))
  (returns (ReturnValue :type "Vector Structure"))
  (bind _spline (`self.Spline`))
  (return (`SplineComponent.GetLocationAtDistanceAlongSpline` _spline (+ (`SplineComponent.GetDistanceAlongSplineAtLocation` _spline (`self.K2_GetActorLocation` Requester) "World") (`KismetMathLibrary.MapRangeClamped` (* (`ChaosVehicleMovementComponent.GetForwardSpeed` (`self.GetComponentByClass` (`local.Requester`) "/Script/ChaosVehicles.ChaosVehicleMovementComponent")) 0.036) 50.0 230.0 1000.0 3000.0)) "World")))

(fn `UserConstructionScript`)